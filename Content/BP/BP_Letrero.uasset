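; BP_Letrero is a sign actor that shows a board once no actors tagged "Pollito" remain in the level.
; Tick polls for that tag and, behind a DoOnce, clears all widgets and blends the player's view to the sign.
; It then builds a WBP_Tablon with the level name, places it on its Widget component, shows the cursor and switches input to Game and UI.
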(event `self.ReceiveTick`
  (params (DeltaSeconds :type "Float (single-precision)"))
  (bind _returnvalue (`GameplayStatics.GetPlayerController` 0))
  (bind _widget (`self.Widget`))
  (bind _outactors (`GameplayStatics.GetAllActorsWithTag` "Pollito"))
  (if (<= (`KismetArrayLibrary.Array_Length` _outactors) 0)
    (`/Engine/EditorBlueprintResources/StandardMacros.DoOnce` false
      (:`Completed`
        (`WidgetLayoutLibrary.RemoveAllWidgets`)
        (`PlayerController.SetViewTargetWithBlend` _returnvalue self 1.0 "VTBlend_EaseInOut" 1.0 false)
        (bind _returnvalue_2 (`|GenericCreateObject` _widget "/Game/WIDGET/WBP_Tablon.WBP_Tablon_C" (`self.Level Name`)))
        (`WidgetComponent.SetWidget` _widget _returnvalue_2)
        (set `PlayerController.bShowMouseCursor` true _returnvalue)
        (`WidgetBlueprintLibrary.SetInputMode_GameAndUIEx` _returnvalue _returnvalue_2)))))

(fn `UserConstructionScript`)